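; BP_Timer is a countdown timer actor that destroys itself when its time runs out.
; StartTimer stores the duration and activates the countdown, which Tick decrements by delta time while printing the remaining time on screen.
; Once the time drops below zero, Tick deactivates the timer and calls OnTimerFinished.
; PauseTimer and ResumeTimer are inverted relative to their names: pause sets the active flag, resume clears it.
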(event `StartTimer`
  (params (Duration :type "Float (double-precision)"))
  (`|ExecutionSequence`
    (:`then_0`
      (set `self.TimeDuration` Duration))
    (:`then_1`
      (set `self.IsTimerActive` true))
    (:`then_2`
      (set `self.RemainingTime` Duration))))

(event `PauseTimer`
  (set `self.IsTimerActive` true))

(event `ResumeTimer`
  (set `self.IsTimerActive` false))

(event `self.ReceiveTick`
  (params (DeltaSeconds :type "Float (single-precision)"))
  (bind _remainingtime (`self.RemainingTime`))
  (if (`self.IsTimerActive`)
    (`|ExecutionSequence`
      (:`then_0`
        (if (>= _remainingtime 0.0)
          (set `self.RemainingTime` (- _remainingtime DeltaSeconds))
          (else
            (`|ExecutionSequence`
              (:`then_0`
                (set `self.IsTimerActive` false))
              (:`then_1`
                (`self.OnTimerFinished`))))))
      (:`then_1`
        (`KismetSystemLibrary.PrintString` (`KismetStringLibrary.Conv_DoubleToString` _remainingtime) true true (struct :`G` 0.66 :`B` 1.0 :`A` 1.0) 0.0)))))

(event `OnTimerFinished`
  (`self.K2_DestroyActor`))

(fn `UserConstructionScript`)