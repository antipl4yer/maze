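; Teleporter Blueprint that glides a given actor from one location to another over a fixed one-second duration.
; A custom event takes the actor and both endpoints, resets the timer and raises flags that start the move.
; Tick then lerps the actor's location without sweeping and, once time is up, re-enables its collision and clears the flags.
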(event `CustomEvent`
  (params (MoveTo :type "Vector Structure") (Actor :type "/Game/Characters/myChar Object Reference") (MoveFrom :type "Vector Structure"))
  (set `self.MoveDuration` 1.0)
  (set `self.TimeElapsed` 0.0)
  (set `self.Fl` true)
  (set `self.Flag` true))

(event `self.ReceiveTick`
  (params (DeltaSeconds :type "Float (single-precision)"))
  (bind _timeelapsed (`self.TimeElapsed`))
  (bind _moveduration (`self.MoveDuration`))
  (if (`self.Flag`)
    (if (< _timeelapsed _moveduration)
      (set `self.TimeElapsed` (+ DeltaSeconds _timeelapsed))
      (`self.K2_SetActorLocation` (stale `CustomEvent` Actor) (`KismetMathLibrary.VLerp` (stale `CustomEvent` MoveFrom) (stale `CustomEvent` MoveTo) (/ _timeelapsed _moveduration)) false false)
      (elif (`self.Fl`)
        (`self.SetActorEnableCollision` (stale `CustomEvent` Actor) true)
        (set `self.Fl` false)
        (set `self.Flag` false)))))

(fn `UserConstructionScript`)